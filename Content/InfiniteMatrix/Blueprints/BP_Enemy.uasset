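; BP_Enemy is an enemy actor that can be shot down by lasers or hurt the player on contact.
; A sphere overlap with BP_Laser destroys both actors and increments the player's score once.
; A player overlap updates the health widget once, and at zero health flags death, shows restart and resets the score.
; RandomizeEnemyLocation, not called here, scatters the mesh in local Y/Z using independently randomized trigonometric offsets.
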(event OnComponentBeginOverlap(SphereCollision)
  (params (OverlappedComponent :type Primitive%20Component%20Object%20Reference) (OtherActor :type Actor%20Object%20Reference) (OtherComp :type Primitive%20Component%20Object%20Reference) (OtherBodyIndex :type Integer) (bFromSweep :type Boolean) (SweepResult :type Hit%20Result%20Structure%20%28by%20ref%29))
  (bind _asbp_laser (Utilities|Casting|CastToBP_Laser OtherActor)
    (:then
      (Actor|DestroyActor)
      (Actor|DestroyActor _asbp_laser)
      (bind _asbp_player (Utilities|Casting|CastToBP_Player (Game|Player|GetPlayerPawn 0)))
      (Utilities|FlowControl|DoOnce false
        (:Completed
          (Default|IncrementScore (Variables|/Game/InfiniteMatrix/Blueprints/BP_Player.BP_Player_C|GetScoreWidget _asbp_player)))))
    (:CastFailed
      (bind _asbp_player_2 (Utilities|Casting|CastToBP_Player OtherActor))
      (Utilities|FlowControl|DoOnce false
        (:Completed
          (Default|Health- (Variables|/Game/InfiniteMatrix/Blueprints/BP_Player.BP_Player_C|GetHealthWidget _asbp_player_2) 2e+01)
          (if (== (Variables|/Game/InfiniteMatrix/UI/WB_Healthbar.WB_Healthbar_C|GetCurrent%20health (Variables|/Game/InfiniteMatrix/Blueprints/BP_Player.BP_Player_C|GetHealthWidget _asbp_player_2)) 0.0)
            (Variables|/Game/InfiniteMatrix/Blueprints/BP_Player.BP_Player_C|SetIsDead _asbp_player_2 (== (Variables|/Game/InfiniteMatrix/UI/WB_Healthbar.WB_Healthbar_C|GetCurrent%20health (Variables|/Game/InfiniteMatrix/Blueprints/BP_Player.BP_Player_C|GetHealthWidget _asbp_player_2)) 0.0))
            (Default|DisplayRestart _asbp_player_2)
            (Default|ResetScore (Variables|/Game/InfiniteMatrix/Blueprints/BP_Player.BP_Player_C|GetScoreWidget _asbp_player_2))))))))

(event EventBeginPlay)

(event Collision|EventActorBeginOverlap
  (params (OtherActor :type Actor%20Object%20Reference)))

(event EventTick
  (params (DeltaSeconds :type Float%20%28single-precision%29)))

(fn ConstructionScript)

(fn RandomizeEnemyLocation
  (bind _returnvalue (Math|Random|RandomFloatinRange 0.0 1.0))
  (bind _returnvalue_2 (Math|Random|RandomFloatinRange 0.0 3.6e+02))
  (bind _returnvalue_3 (Math|Trig|DegreesToRadians _returnvalue_2))
  (bind _returnvalue_4 (Math|Float|Sqrt _returnvalue))
  (bind _returnvalue_5 (* _returnvalue_4 4e+02))
  (Transformation|AddLocalOffset (Variables|Default|GetEnemyMesh) (Math|Vector|MakeVector 0.0 (* (Math|Trig|Cos(Radians) _returnvalue_3) _returnvalue_5) (* (Math|Trig|Sin(Radians) _returnvalue_3) _returnvalue_5)) false false))